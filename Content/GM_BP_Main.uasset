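; Main game mode for a cellular-automaton board game, switching between a board creation phase and a simulation phase, each with its own widget.
; BeginPlay finds the visualization controller, sets a static camera and forwards player controller pan requests to the visualization.
; StartSimulation seeds a max-size board with live cells.
; Tick advances one generation per frame while simulating and unpaused, and refreshes the visualization every frame regardless of phase.
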(event `self.ReceiveBeginPlay`
  (`|ExecutionSequence`
    (:`then_0`
      (bind _returnvalue (`GameplayStatics.GetActorOfClass` "/Game/Actor_BP_BoardVisualizationController.Actor_BP_BoardVisualizationController_C"))
      (set `self.VisualizationController` _returnvalue))
    (:`then_1`
      (bind _returnvalue_2 (`|CreateWidget` "/Game/WBP_BoardCreation.WBP_BoardCreation_C"))
      (set `self.BoardCreationWidget` _returnvalue_2)
      (bind _returnvalue_3 (`|CreateWidget` "/Game/WBP_Simulation.WBP_Simulation_C"))
      (set `self.SimulationWidget` _returnvalue_3)
      (bind _returnvalue_4 (`GameplayStatics.GetActorOfClass` "/Game/Camera_BP_StaticBoardCamera.Camera_BP_StaticBoardCamera_C"))
      (`PlayerController.SetViewTargetWithBlend` (`GameplayStatics.GetPlayerController` 0) _returnvalue_4 0.0 "VTBlend_Linear" 0.0 false))
    (:`then_2`
      (`self.GoToCreationPhase`))
    (:`then_3`
      (bind _asplayer_controller_bp_main (cast `/Game/PlayerController_BP_Main` (`GameplayStatics.GetPlayerController` 0)))
      (add `/Game/PlayerController_BP_Main.RequestPanUp` _asplayer_controller_bp_main (delegate `Pan Up`))
      (add `/Game/PlayerController_BP_Main.RequestPanLeft` _asplayer_controller_bp_main (delegate `Pan Left`))
      (add `/Game/PlayerController_BP_Main.RequestPanRight` _asplayer_controller_bp_main (delegate `Pan Right`))
      (add `/Game/PlayerController_BP_Main.RequestPanDown` _asplayer_controller_bp_main (delegate `Pan Down`)))))

(event `Pan Up`
  (`/Game/Actor_BP_BoardVisualizationController.Pan Up` (`self.VisualizationController`)))

(event `Pan Left`
  (`/Game/Actor_BP_BoardVisualizationController.Pan Left` (`self.VisualizationController`)))

(event `Pan Right`
  (`/Game/Actor_BP_BoardVisualizationController.Pan Right` (`self.VisualizationController`)))

(event `Pan Down`
  (`/Game/Actor_BP_BoardVisualizationController.Pan Down` (`self.VisualizationController`)))

(event `self.ReceiveTick`
  (params (DeltaSeconds :type "Float (single-precision)"))
  (bind _gameboard (`self.GameBoard`))
  (if (`self.ShouldSimulate`)
    (`GameBoard.SimulateNextGeneration` _gameboard))
  (`/Game/Actor_BP_BoardVisualizationController.UpdateVisualization` (`self.VisualizationController`) _gameboard))

(event `StartSimulation`
  (params (CoordinatesToStartAlive :type "Array of BoardCoordinate Structure"))
  (bind _returnvalue (`GameBoard.InitializeMaxSizeBoard`))
  (set `self.GameBoard` _returnvalue)
  (for _array_element CoordinatesToStartAlive
    (`GameBoard.SetCellToAlive` (`self.GameBoard`) _array_element))
  (`/Game/Actor_BP_BoardVisualizationController.UpdateVisualization` (`self.VisualizationController`) (`self.GameBoard`))
  (`self.GoToSimulationPhase`))

(event `TogglePauseSimulation`
  (set `self.IsPaused` (not (`self.IsPaused`))))

(event `ResetBoard`
  (`self.GoToCreationPhase`))

(fn `GoToCreationPhase`
  (set `self.IsInSimulationPhase` false)
  (`/Game/Actor_BP_BoardVisualizationController.ResetVisualization` (`self.VisualizationController`))
  (`Widget.RemoveFromParent` (`self.SimulationWidget`))
  (`UserWidget.AddToViewport` (`self.BoardCreationWidget`) 0))

(fn `GoToSimulationPhase`
  (set `self.IsInSimulationPhase` true)
  (set `self.IsPaused` false)
  (`Widget.RemoveFromParent` (`self.BoardCreationWidget`))
  (`UserWidget.AddToViewport` (`self.SimulationWidget`) 0))

(fn `ShouldSimulate`
  (returns (ShouldSimulate :type Boolean))
  (return (and (`self.IsInSimulationPhase`) (not (`self.IsPaused`)))))

(fn `UserConstructionScript`)